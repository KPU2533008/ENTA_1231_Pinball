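; Flipper actor, apparently pinball-style, that swings its mesh when activated, with a Direction setting choosing the side.
; Construction flips the anchor 180 degrees by Direction, which also sets the swing's sign.
; Async physics tick springs Alpha toward that signed target, or zero when inactive, and applies it as swept mesh yaw.
; SetFlipperActive sets the state and swaps in a sticky physical material while active.
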(event `self.ReceiveAsyncPhysicsTick`
  (params (DeltaSeconds :type "Float (single-precision)") (SimSeconds :type "Float (single-precision)"))
  (bind _returnvalue (`KismetMathLibrary.FloatSpringInterp` (`self.Alpha`) (`KismetMathLibrary.SelectFloat` (`KismetMathLibrary.SelectFloat` -1.0 1.0 (`|EnumEquality` (`self.Direction`) "NewEnumerator0")) 0.0 (`self.IsActive`)) (`self.SpringState`) 0.85 1.2 DeltaSeconds 0.003 0.8))
  (bind _output_get (set `self.Alpha` _returnvalue))
  (`SceneComponent.K2_SetRelativeRotation` (`self.FlipperMesh`) (`KismetMathLibrary.MakeRotator` 0.0 0.0 (* _output_get 60.0)) true false))

(fn `SetFlipperActive`
  (params (Active :type Boolean))
  (set `self.IsActive` Active)
  (`PrimitiveComponent.SetPhysMaterialOverride` (`self.FlipperMesh`) (select `bool` Active :`false` "/Game/Materials/PM_Flipper.PM_Flipper" :`true` "/Game/Materials/PM_FlipperSticky.PM_FlipperSticky" :!type "PhysicalMaterial Object Reference")))

(fn `UserConstructionScript`
  (`SceneComponent.K2_SetRelativeRotation` (`self.FlipperAnchor`) (`KismetMathLibrary.SelectRotator` (struct :`Yaw` 180.0) (struct) (`|EnumEquality` (`self.Direction`) "NewEnumerator0")) true false))