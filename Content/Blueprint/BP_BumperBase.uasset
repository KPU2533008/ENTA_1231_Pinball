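; BP_BumperBase is a base pinball bumper that launches objects that hit it.
; On Hit, it casts the other actor to BPI_PinballReactive and calls PinballApplyImpulse with a direction scaled by BumpForce.
; UseHitNormal chooses between the hit normal and the normalized vector from the bumper component to the other component.
; A debug string prints on each launch, and the construction script is empty.
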(event `self.ReceiveHit`
  (params (MyComp :type "PrimitiveComponent Object Reference") (Other :type "Actor Object Reference") (OtherComp :type "PrimitiveComponent Object Reference") (bSelfMoved :type Boolean) (HitLocation :type "Vector Structure") (HitNormal :type "Vector Structure") (NormalImpulse :type "Vector Structure") (Hit :type "HitResult Structure (by ref)"))
  (bind _asbpi_pinball_reactive (cast `/Game/Interface/BPI_PinballReactive` Other))
  (`/Game/Interface/BPI_PinballReactive.PinballApplyImpulse` _asbpi_pinball_reactive (* (`KismetMathLibrary.SelectVector` HitNormal (`KismetMathLibrary.Normal` (- (`SceneComponent.K2_GetComponentLocation` OtherComp) (`SceneComponent.K2_GetComponentLocation` MyComp))) (`self.UseHitNormal`)) (`self.BumpForce`)))
  (`KismetSystemLibrary.PrintString` "launch ball"))

(fn `UserConstructionScript`)