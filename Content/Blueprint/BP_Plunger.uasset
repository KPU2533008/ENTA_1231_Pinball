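; Pinball plunger that pulls back while held and launches the balls in its lane on release.
; An overlap volume tracks captured BPI_PinballReactive balls, and Pull and Release toggle charging and store launch force from pullback.
; Async physics tick ramps the pullback and animates the mesh through a spring interp.
; Once the released spring nears rest, it sets each captured ball's velocity along the plunger's negative right axis, once per pull.
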(event `self.ReceiveBeginPlay`
  (bind _pinballcapture (`self.PinballCapture`))
  (add `PrimitiveComponent.OnComponentBeginOverlap` _pinballcapture (delegate `Event OnPinballCaptured`))
  (add `PrimitiveComponent.OnComponentEndOverlap` _pinballcapture (delegate `Event OnPinballReleased`)))

(event `Event OnPinballCaptured`
  (params (OverlappedComponent :type "PrimitiveComponent Object Reference") (OtherActor :type "Actor Object Reference") (OtherComp :type "PrimitiveComponent Object Reference") (OtherBodyIndex :type Integer) (bFromSweep :type Boolean) (SweepResult :type "HitResult Structure (by ref)"))
  (bind _asbpi_pinball_reactive (cast `/Game/Interface/BPI_PinballReactive` OtherActor))
  (`KismetArrayLibrary.Array_Add` (`self.CapturedPinballs`) _asbpi_pinball_reactive))

(event `Event OnPinballReleased`
  (params (OverlappedComponent :type "PrimitiveComponent Object Reference") (OtherActor :type "Actor Object Reference") (OtherComp :type "PrimitiveComponent Object Reference") (OtherBodyIndex :type Integer))
  (bind _asbpi_pinball_reactive (cast `/Game/Interface/BPI_PinballReactive` OtherActor))
  (`KismetArrayLibrary.Array_RemoveItem` (`self.CapturedPinballs`) _asbpi_pinball_reactive))

(event `self.ReceiveAsyncPhysicsTick`
  (params (DeltaSeconds :type "Float (single-precision)") (SimSeconds :type "Float (single-precision)"))
  (bind (_pullbackalpha _animatedpullback) (`self.StepPullback` DeltaSeconds))
  (`SceneComponent.K2_SetRelativeLocation` (`self.SM_Plunger`) (* (0.0 100.0 0.0) _animatedpullback) false false)
  (if (and (not (`self.Launched`)) (< (`self.AnimatedAlpha`) 0.05) (not (`self.IsPulling`)))
    (for _array_element (`self.CapturedPinballs`)
      (`/Game/Interface/BPI_PinballReactive.PinballSetVelocity` _array_element (* (`KismetMathLibrary.GetRightVector` (`SceneComponent.K2_GetComponentRotation` (`self.SM_Plunger`))) (`self.LastLaunchForce`) -1.0)))
    (set `self.Launched` true)))

(fn `Pull`
  (if (== (`self.AnimatedAlpha`) 0.0)
    (set `self.IsPulling` true)
    (set `self.Launched` false)))

(fn `Release`
  (set `self.LastLaunchForce` (* (`self.PullbackAlpha`) (`self.MaxForce`)))
  (set `self.IsPulling` false))

(fn `StepPullback`
  (params (DeltaTime :type "Float (double-precision)"))
  (returns (PullbackAlpha :type "Float (double-precision)") (AnimatedPullback :type "Float (double-precision)"))
  (bind _output_get (set `self.PullbackAlpha` (`KismetMathLibrary.FClamp` (`KismetMathLibrary.SelectFloat` (+ (`self.PullbackAlpha`) (* DeltaTime 0.85)) 0.0 (`self.IsPulling`)))))
  (bind _returnvalue (`KismetMathLibrary.FloatSpringInterp` (`self.AnimatedAlpha`) _output_get (`self.PullbackSpring`) 0.85 1.1 DeltaTime 0.0055 0.8 true 0.0))
  (bind _output_get_2 (set `self.AnimatedAlpha` _returnvalue))
  (return _output_get _output_get_2))

(fn `UserConstructionScript`)