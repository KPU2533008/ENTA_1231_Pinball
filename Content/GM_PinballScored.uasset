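; Pinball game mode that adds scoring and lives on top of a parent game mode.
; AddScore forwards points to BP_PinballGameState.
; OnBallLost runs the parent logic, decrements the game state's Lives, and spawns a new pinball only while lives remain.
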(event `/Game/Blueprint/Interface/BPI_ScoreReceiver.AddScore`
  (params (Points :type Integer))
  (bind _asbp_pinball_game_state (cast `/Game/BP_PinballGameState` (`GameplayStatics.GetGameState`)))
  (`/Game/BP_PinballGameState.AddScore` _asbp_pinball_game_state Points))

(event `self.OnBallLost`
  (`parent.OnBallLost`)
  (bind _asbp_pinball_game_state (cast `/Game/BP_PinballGameState` (`GameplayStatics.GetGameState`)))
  (`/Game/BP_PinballGameState.SetLives` _asbp_pinball_game_state (- (`/Game/BP_PinballGameState.Lives` _asbp_pinball_game_state) 1))
  (if (> (`/Game/BP_PinballGameState.Lives` _asbp_pinball_game_state) 0)
    (`self.SpawnPinball`)))

(fn `UserConstructionScript`
  (`parent.UserConstructionScript`))