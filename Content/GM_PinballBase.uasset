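; Base pinball game mode that owns the current ball and handles its spawning and removal.
; SetPinballSpawn takes effect only once, storing the spawn position and calling SpawnPinball.
; SpawnPinball destroys any existing ball, then spawns a PinballClass actor at the stored position and tracks it as CurrentPinball.
; OnBallLost destroys the current ball without spawning a replacement.
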(event `OnBallLost`
  (bind _currentpinball (`self.CurrentPinball`))
  (`/Engine/EditorBlueprintResources/StandardMacros.IsValid` _currentpinball
    (:`Is Valid`
      (`self.K2_DestroyActor` _currentpinball))))

(event `SetPinballSpawn`
  (params (SpawnPosition :type "Vector Structure"))
  (`/Engine/EditorBlueprintResources/StandardMacros.DoOnce` false
    (:`Completed`
      (set `self.PinballSpawnPosition` SpawnPosition)
      (`self.SpawnPinball`))))

(fn `SpawnPinball`
  (bind _currentpinball (`self.CurrentPinball`))
  (`|ExecutionSequence`
    (:`then_0`
      (`/Engine/EditorBlueprintResources/StandardMacros.IsValid` _currentpinball
        (:`Is Valid`
          (`self.K2_DestroyActor` _currentpinball)
          (set `self.CurrentPinball` null))))
    (:`then_1`
      (bind _returnvalue (`|SpawnActorFromClass` (`self.PinballClass`) (`KismetMathLibrary.MakeTransform` (`self.PinballSpawnPosition`)) "Undefined" "MultiplyWithRoot" null null))
      (set `self.CurrentPinball` _returnvalue))))

(fn `UserConstructionScript`)